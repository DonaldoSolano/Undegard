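; Player character Blueprint that supports either a first-person or third-person view and shows a sight widget on screen.
; The construction script uses UseFirstPersonView to set auto-activation on either the FPS camera or the TPS camera and spring arm.
; BeginPlay adds the BP_Sight widget to the viewport.
; Melee detector overlaps and the CharacterActionDebug event only print debug strings, with no gameplay effect in this graph.
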(event OnComponentBeginOverlap(MeleeDetectorComponent)
  (params (OverlappedComponent :type Primitive%20Component%20Object%20Reference) (OtherActor :type Actor%20Object%20Reference) (OtherComp :type Primitive%20Component%20Object%20Reference) (OtherBodyIndex :type Integer) (bFromSweep :type Boolean) (SweepResult :type Hit%20Result%20Structure%20%28by%20ref%29))
  (Development|PrintString (Utilities|GetDisplayName OtherActor)))

(event EventBeginPlay
  (bind _returnvalue (UserInterface|CreateWidget "/Game/Widgets/BP_Sight.BP_Sight_C"))
  (UserInterface|Viewport|AddtoViewport _returnvalue 0))

(event Collision|EventActorBeginOverlap
  (params (OtherActor :type Actor%20Object%20Reference)))

(event EventTick
  (params (DeltaSeconds :type Float%20%28single-precision%29)))

(event EventCharacterActionDebug
  (Development|PrintString "Action is happening:Checking boolean"))

(fn ConstructionScript
  (Components|Activation|SetAutoActivate (Variables|Default|GetFPSCameraComponent) (Variables|Default|GetbUseFirstPersonView))
  (Components|Activation|SetAutoActivate (Variables|Default|GetTPSCameraComponent) (not (Variables|Default|GetbUseFirstPersonView))))